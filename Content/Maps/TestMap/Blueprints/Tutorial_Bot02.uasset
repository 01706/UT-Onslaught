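; Tutorial bot pawn that self-possesses with an AIController and serves as a target that can taunt, patrol or guard a token cage.
; Timers drive random taunts and movement alternating between two patrol points.
; On death it optionally respawns as a taunting Tutorial_Bot01, or notifies its registered token cage and pops its glowing sphere, then destroys itself.
; Helmet-giving logic exists but is disconnected.
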(event `/Game/RestrictedAssets/Tutorials/Blueprints/BPI_TargetDummy.RegisterTokenCage`
  (params (TokenCage :type "Actor Object Reference"))
  ;[1 1 1] receive token cage ref
  (set `self.MyTokenCage` TokenCage))

(event `OnDied_Event_0` :!signature `self.OnDied`
  (params (Killer :type "Controller Object Reference") (DamageType :type "DamageType Object Reference"))
  (bind _returnvalue (`SceneComponent.K2_GetComponentLocation` (`self.SM_Sphere`)))
  ;[1 1 1] bind OnDied
  (if (`self.bRespawnOnDeath`)
    ;[1 1 1] respawn on death
    (`KismetSystemLibrary.Delay` 0.5)
    (bind _returnvalue_2 (`|SpawnActorFromClass` "/Game/RestrictedAssets/Tutorials/Blueprints/Tutorial_Bot01.Tutorial_Bot01_C" (`KismetMathLibrary.MakeTransform` (`SceneComponent.K2_GetComponentLocation` (`self.SpawnLocation`))) "AdjustIfPossibleButDontSpawnIfColliding" "OverrideRootScale" null true false true))
    (`self.SpawnDefaultController` _returnvalue_2))
  (if (`self.bTokenCageDummy`)
    ;[1 1 1] notify token cage
    (message `/Game/RestrictedAssets/Tutorials/Blueprints/BPI_TargetDummy.TargetDummyDestroyed` (`self.MyTokenCage`) self)
    ;[1 1 1] spawn fx
    (bind _returnvalue_3 (`GameplayStatics.SpawnEmitterAtLocation` "/Game/RestrictedAssets/Tutorials/FX/PS_GlowySphere_Poof.PS_GlowySphere_Poof" _returnvalue))
    (`SceneComponent.DetachFromParent` _returnvalue_3 true true)
    (`GameplayStatics.PlaySoundAtLocation` "/Game/RestrictedAssets/Audio/Gameplay/A_Powerup_Invulnerability_Pickup_Cue.A_Powerup_Invulnerability_Pickup_Cue" _returnvalue (struct) 1.2 0.8)
    (`ActorComponent.K2_DestroyComponent` (`self.GlowyLight`))
    (`ActorComponent.K2_DestroyComponent` (`self.SM_Sphere`)))
  ;[1 1 1] clean up
  (`KismetSystemLibrary.Delay` 1.0)
  (`self.K2_DestroyActor`))

(event `self.ReceiveBeginPlay`
  ;[1 1 1] beginplay
  (`parent.ReceiveBeginPlay`)
  ;[1 1 1] spawn ai controller
  (bind _returnvalue (`|SpawnActorFromClass` "/Script/AIModule.AIController" (`self.GetTransform`) "AlwaysSpawn" "OverrideRootScale"))
  (`Controller.Possess` _returnvalue self)
  ;[1 1 1] play spawn FX
  (`GameplayStatics.SpawnEmitterAtLocation` "/Game/RestrictedAssets/Effects/TomB/P_Player_Spawn.P_Player_SPawn" (`self.K2_GetActorLocation`))
  (`|ExecutionSequence`
    (:`then_0`
      ;[1 1 1] bind OnDied
      (add `self.OnDied` (delegate `OnDied_Event_0`)))
    (:`then_1`
      ;[1 1 1] set taunt timer
      (if (and (`self.bAutoTaunt`) (not (`self.bIsPatrolling`)))
        (`self.SetTauntTimer`)))
    (:`then_2`
      ;[1 1 1] activate glowy sphere FX?
      (if (`self.bTokenCageDummy`)
        (`ActorComponent.SetActive` (`self.PS_GlowySphere`) true false)))
    (:`then_4`
      ;[1 1 1] are we patrolling?
      (if (`self.bIsPatrolling`)
        (if (`self.bAutoTaunt`)
          (`self.PlayTauntMontage`)
          (else
            (`self.Patrol`)))))))

(fn `GiveHelmet`
  (if (`self.bGiveHelmet`)
    (bind _returnvalue (`|SpawnActorFromClass` "/Game/RestrictedAssets/Pickups/Armor/Armor_ThighPads.Armor_ThighPads_C" (`KismetMathLibrary.MakeTransform` (0.0 0.0 0.0)) "AdjustIfPossibleButDontSpawnIfColliding" "OverrideRootScale"))
    (`self.AddInventory` _returnvalue true)))

(fn `Patrol`
  (if (`self.bAutoTaunt`)
    (`self.SetTauntTimer`)
    (bind _returnvalue (`self.GetCurrentMontage`))
    (`self.StopAnimMontage` _returnvalue)
    (else
      (`self.SetPatrolTimer`)))
  (`NavigationSystem.SimpleMoveToLocation` (`self.GetController`) (select `bool` (`self.bPatrolRouteA`) :`false` (`self.PatrolPointB`) :`true` (`self.PatrolPointA`)))
  (if (`self.bPatrolRouteA`)
    (set `self.bPatrolRouteA` false)
    (else
      (set `self.bPatrolRouteA` true))))

(fn `PlayTauntMontage`
  (bind _tauntlist (`self.TauntList`))
  (if (`self.bIsPatrolling`)
    (`MovementComponent.StopMovementImmediately`))
  (`self.PlayTauntByClass` (`|GetArrayItem` _tauntlist (`KismetMathLibrary.RandomIntegerInRange` 0 (`KismetArrayLibrary.Array_LastIndex` _tauntlist))))
  (if (`self.bIsPatrolling`)
    (`KismetSystemLibrary.K2_SetTimer` null "Patrol" (`KismetMathLibrary.RandomFloatInRange` (`self.TauntTimerMin`) (`self.TauntTimerMax`)))
    (else
      (`self.SetTauntTimer`)))
  (return))

(fn `SetPatrolTimer`
  (`KismetSystemLibrary.K2_SetTimer` null "Patrol" (`KismetMathLibrary.RandomFloatInRange` (`self.PatrolTimerMin`) (`self.PatrolTimerMax`)))
  (return))

(fn `SetTauntTimer`
  (bind _taunttimermax (`self.TauntTimerMax`))
  (`KismetSystemLibrary.K2_SetTimer` null "PlayTauntMontage" (`KismetMathLibrary.RandomFloatInRange` (`self.TauntTimerMin`) (`KismetMathLibrary.SelectFloat` (* _taunttimermax 0.5) _taunttimermax (`self.bIsPatrolling`))))
  (return))

(fn `UserConstructionScript`
  (`parent.UserConstructionScript`)
  (`SceneComponent.DetachFromParent` (`self.SpawnLocation`) true true)
  (if (`self.bTokenCageDummy`)
    (`SceneComponent.SetHiddenInGame` (`self.SM_Sphere`) false false)
    (`LightComponent.SetIntensity` (`self.GlowyLight`) 2500.0)))