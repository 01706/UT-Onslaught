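; BP_NodeEnhancement_Bridge is a bridge enhancement for an Onslaught node objective, set up in a test map.
; SetControllingNode casts the objective, stores it as ControlNode and adds the bridge to that node's Enhancements list, with debug prints along the way.
; Activation plays a timeline that rolls the Arrow component by the negated Opening value, and deactivation reverses it to swing the Arrow back.
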(event `UTOnslaughtEnhancementInterface.SetControllingNode`
  (params (NewObjective :type "Actor Object Reference"))
  (`KismetSystemLibrary.PrintString` "SetControllingNode Called on Bridge")
  (bind _asutonslaught_node_objective (cast `UTOnslaughtNodeObjective` NewObjective)
    (:`then`
      (`KismetSystemLibrary.PrintString` "Bridge setting ControlNode")
      (set `self.ControlNode` _asutonslaught_node_objective)
      (`KismetArrayLibrary.Array_Add` (`UTOnslaughtNodeObjective.Enhancements` _asutonslaught_node_objective) self))
    (:`CastFailed`
      (`KismetSystemLibrary.PrintString` "bridge cast failed ..."))))

(event `UTOnslaughtEnhancementInterface.ActivateEnhancement`
  (bind (_direction _opening) (`Timeline|Timeline_0` :!label _label)
    (:`Update`
      (`SceneComponent.K2_SetRelativeRotation` (`self.Arrow`) (`KismetMathLibrary.MakeRotator` (* _opening -1.0)) false false))))

(event `UTOnslaughtEnhancementInterface.DeactivateEnhancement`
  (goto _label :!via `Reverse`))

(fn `GetControllingNode`
  (returns (ReturnValue :type "Actor Object Reference"))
  (return (`self.ControlNode`)))

(fn `UserConstructionScript`)