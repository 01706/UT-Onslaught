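; BP_Onslaught_Node is a node actor for an Onslaught mode, with its gameplay logic apparently left to its parent class.
; The construction script toggles the OrbRadius capsule by ShowInvulnerableRadius and sizes it to InvulnerableRadius when shown, previewing that radius.
; BeginPlay and Tick are empty.
; Disconnected leftovers include a destruction burst, a beam color parameter write and team-based shield tinting, none of which runs.
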(event `self.ReceiveBeginPlay`)

(event `self.ReceiveTick`
  (params (DeltaSeconds :type "Float (single-precision)")))

(fn `UserConstructionScript`
  (bind _invulnerableradius (`self.InvulnerableRadius`))
  (bind _orbradius (`self.OrbRadius`))
  (if (`self.bShowInvulnerableRadius`)
    (`SceneComponent.SetVisibility` _orbradius true false)
    (`CapsuleComponent.SetCapsuleSize` _orbradius _invulnerableradius _invulnerableradius false)
    (else
      (`SceneComponent.SetVisibility` _orbradius false false))))