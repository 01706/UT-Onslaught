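; BP_Onslaught_PowerCore is an Onslaught power core actor with a core, base and team-coloured beam.
; The construction script tints the beam through a dynamic material and sets the base material by TeamNum, using temporary lookup arrays instead of UTTeamGame colours.
; Team 255 gets a default beam colour and keeps its base material.
; Zero-health destruction logic (hide, disable collision, spawn explosion) exists but is unconnected, so it never runs.
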(fn `UserConstructionScript`
  (bind _returnvalue (`KismetMathLibrary.Conv_ByteToInt` (`self.TeamNum`)))
  (bind _returnvalue_2 (== _returnvalue 255))
  (bind _returnvalue_3 (`PrimitiveComponent.CreateDynamicMaterialInstance` (`self.TeamBeam`) 0 null))
  (bind _output_get (set `self.M_TowerBeamInstance` _returnvalue_3))
  (if _returnvalue_2
    (`MaterialInstanceDynamic.SetVectorParameterValue` _output_get "TeamColour" (make `LinearColor` 0.0))
    (else
      ;[1 1 1] Set TeamBeam colour
      (`MaterialInstanceDynamic.SetVectorParameterValue` _output_get "TeamColour" (`KismetArrayLibrary.Array_Get` (`self.TempTeamColours`) _returnvalue))))
  (if (not _returnvalue_2)
    ;[1 1 1] Set Base Materal
    (`PrimitiveComponent.SetMaterial` (`self.Base`) 0 (`KismetArrayLibrary.Array_Get` (`self.TempTeamMaterial`) _returnvalue))))